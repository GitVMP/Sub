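; Atlantic torpedo environment piece that moves along a spline and offers an interact widget to the player's FlyingPawn.
; On BeginPlay, a timeline drives the scene component along the spline, aiming it at a point slightly ahead.
; Tick turns the widget toward the pawn's camera, reveals whichever widget its WidgetInteraction hovers, hides the torpedo's otherwise, and updates HoveringAWidget.
; The delayed fish-hit sound is disconnected and never plays.
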(event EventBeginPlay
  (bind _spline (Variables|Default|GetSpline))
  ;[1 1 1] Get a reference to flying pawn and run torpedo along spline
  (bind _asflying_pawn (Utilities|Casting|CastToFlyingPawn (Game|Player|GetPlayerPawn 0)))
  (Variables|Default|SetFlyingPawnReference _asflying_pawn)
  (bind _animation_of_atlantic_torpedo_on_path (Timeline|Timeline_0 PlayFromStart)
    (:Update
      (Transformation|SetWorldTransform (Variables|Default|GetScene1) (Math|Transform|MakeTransform (Spline|GetLocationatDistanceAlongSpline _spline (* (Spline|GetSplineLength _spline) _animation_of_atlantic_torpedo_on_path) "World") (Math|Rotator|FindLookatRotation (Spline|GetLocationatDistanceAlongSpline _spline (* (Spline|GetSplineLength _spline) _animation_of_atlantic_torpedo_on_path) "World") (Spline|GetLocationatDistanceAlongSpline _spline (+ (* (Spline|GetSplineLength _spline) _animation_of_atlantic_torpedo_on_path) 2e+01) "World")) "0.500000,0.500000,0.500000") false false)
      (Utilities|FlowControl|DoOnce false))))

(event EventTick
  (params (DeltaSeconds :type Float%20%28single-precision%29))
  (bind _flyingpawnreference (Variables|Default|GetFlyingPawnReference))
  (bind _widgetinteraction (Variables|/Game/FlyingBP/Blueprints/FlyingPawn.FlyingPawn_C|GetWidgetInteraction _flyingpawnreference))
  (bind _returnvalue (Class|WidgetInteractionComponent|GetHoveredWidgetComponent _widgetinteraction))
  ;[1 1 1] Show interact widget when they look at the torpedo and face it towards the player
  (Transformation|SetWorldRotation (Variables|Default|GetInteract_Torpedo) (Math|Rotator|FindLookatRotation (Transformation|GetWorldLocation (Variables|Default|GetInteract_Torpedo)) (Transformation|GetWorldLocation (Variables|/Game/FlyingBP/Blueprints/FlyingPawn.FlyingPawn_C|GetCamera (Variables|Default|GetFlyingPawnReference)))) false false)
  (if (Utilities|Enum|NotEqual(Enum) (Utilities|GetDisplayName _returnvalue) "") ; Check if they are hovering a widget. If yes, display that widget
    (Class|WidgetComponent|SetTintColorandOpacity _returnvalue "(R=1.000000,G=1.000000,B=1.000000,A=1.000000)") ; Show the widget that is being hovered
    (Variables|/Game/FlyingBP/Blueprints/FlyingPawn.FlyingPawn_C|SetHoveringAWidget? (Variables|Default|GetFlyingPawnReference) true)
    (else
      (Class|WidgetComponent|SetTintColorandOpacity (Variables|Default|GetInteract_Torpedo) "(R=0.000000,G=0.000000,B=0.000000,A=0.000000)") ; Hide all widgets that arent being hovered  (Connect all interact components here)
      (Variables|/Game/FlyingBP/Blueprints/FlyingPawn.FlyingPawn_C|SetHoveringAWidget? (Variables|Default|GetFlyingPawnReference) false))))

(fn ConstructionScript)