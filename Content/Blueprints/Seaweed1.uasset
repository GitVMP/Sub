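; Seaweed actor with four seaweed pieces, each with its own box that detects when the player's FlyingPawn leaves it.
; On each end overlap, a single RInterpTo step nudges that piece toward the starting rotation, with no tick or timeline to continue the motion.
; All four share Seaweed1's BeginPlay rotation as target.
; The stored seaweed array and pawn reference go unused here, and nothing here bends the seaweed.
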(event OnComponentEndOverlap(Seaweed1Box)
  (params (OverlappedComponent :type Primitive%20Component%20Object%20Reference) (OtherActor :type Actor%20Object%20Reference) (OtherComp :type Primitive%20Component%20Object%20Reference) (OtherBodyIndex :type Integer))
  ;[1 1 1] Return seaweed 1 to original rotation when they arent touching it
  (Utilities|Casting|CastToFlyingPawn OtherActor)
  (Transformation|SetWorldRotation (Variables|Default|GetSeaweed1) (Math|Interpolation|RInterpTo (Transformation|GetWorldRotation (Variables|Default|GetSeaweed1)) (Variables|Default|GetOriginalRotation) (Utilities|Time|GetWorldDeltaSeconds) 1.0) false false))

(event OnComponentEndOverlap(Seaweed2Box)
  (params (OverlappedComponent :type Primitive%20Component%20Object%20Reference) (OtherActor :type Actor%20Object%20Reference) (OtherComp :type Primitive%20Component%20Object%20Reference) (OtherBodyIndex :type Integer))
  ;[1 1 1] Return seaweed 2 to original rotation when they arent touching it
  (Utilities|Casting|CastToFlyingPawn OtherActor)
  (Transformation|SetWorldRotation (Variables|Default|GetSeaweed2) (Math|Interpolation|RInterpTo (Transformation|GetWorldRotation (Variables|Default|GetSeaweed2)) (Variables|Default|GetOriginalRotation) (Utilities|Time|GetWorldDeltaSeconds) 1.0) false false))

(event OnComponentEndOverlap(Seaweed3Box)
  (params (OverlappedComponent :type Primitive%20Component%20Object%20Reference) (OtherActor :type Actor%20Object%20Reference) (OtherComp :type Primitive%20Component%20Object%20Reference) (OtherBodyIndex :type Integer))
  ;[1 1 1] Return seaweed 3 to original rotation when they arent touching it
  (Utilities|Casting|CastToFlyingPawn OtherActor)
  (Transformation|SetWorldRotation (Variables|Default|GetSeaweed3) (Math|Interpolation|RInterpTo (Transformation|GetWorldRotation (Variables|Default|GetSeaweed3)) (Variables|Default|GetOriginalRotation) (Utilities|Time|GetWorldDeltaSeconds) 1.0) false false))

(event OnComponentEndOverlap(Seaweed4Box)
  (params (OverlappedComponent :type Primitive%20Component%20Object%20Reference) (OtherActor :type Actor%20Object%20Reference) (OtherComp :type Primitive%20Component%20Object%20Reference) (OtherBodyIndex :type Integer))
  ;[1 1 1] Return seaweed 4 to original rotation when they arent touching it
  (Utilities|Casting|CastToFlyingPawn OtherActor)
  (Transformation|SetWorldRotation (Variables|Default|GetSeaweed4) (Math|Interpolation|RInterpTo (Transformation|GetWorldRotation (Variables|Default|GetSeaweed4)) (Variables|Default|GetOriginalRotation) (Utilities|Time|GetWorldDeltaSeconds) 1.0) false false))

(event EventBeginPlay
  (Variables|Default|SetSeaweedArray (Utilities|Array|MakeArray (Variables|Default|GetSeaweed1) (Variables|Default|GetSeaweed2) (Variables|Default|GetSeaweed3) (Variables|Default|GetSeaweed4)))
  (Variables|Default|SetOriginalRotation (Transformation|GetWorldRotation (Variables|Default|GetSeaweed1)))
  (bind _asflying_pawn (Utilities|Casting|CastToFlyingPawn (Game|Player|GetPlayerPawn 0)))
  (Variables|Default|SetFlyingPawnReference _asflying_pawn))

(fn ConstructionScript)