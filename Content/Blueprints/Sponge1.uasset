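; Sponge prop actor with four sponges, each with its own box, that nudges a sponge back toward rest when the FlyingPawn stops overlapping it.
; BeginPlay stores the sponges, the player's FlyingPawn and Sponge1's rotation, which serves as the rest rotation for all four.
; Each end overlap applies a single RInterpTo step toward that rotation, not a continuous return.
; Nothing here rotates the sponges away from rest.
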(event OnComponentEndOverlap(Sponge1Box)
  (params (OverlappedComponent :type Primitive%20Component%20Object%20Reference) (OtherActor :type Actor%20Object%20Reference) (OtherComp :type Primitive%20Component%20Object%20Reference) (OtherBodyIndex :type Integer))
  ;[1 1 1] Return sponge 1 to original rotation when they arent touching it
  (Utilities|Casting|CastToFlyingPawn OtherActor)
  (Transformation|SetWorldRotation (Variables|Default|GetSponge1) (Math|Interpolation|RInterpTo (Transformation|GetWorldRotation (Variables|Default|GetSponge1)) (Variables|Default|GetOriginalRotation) (Utilities|Time|GetWorldDeltaSeconds) 1.0) false false))

(event OnComponentEndOverlap(Sponge2Box)
  (params (OverlappedComponent :type Primitive%20Component%20Object%20Reference) (OtherActor :type Actor%20Object%20Reference) (OtherComp :type Primitive%20Component%20Object%20Reference) (OtherBodyIndex :type Integer))
  ;[1 1 1] Return sponge 2 to original rotation when they arent touching it
  (Utilities|Casting|CastToFlyingPawn OtherActor)
  (Transformation|SetWorldRotation (Variables|Default|GetSponge2) (Math|Interpolation|RInterpTo (Transformation|GetWorldRotation (Variables|Default|GetSponge2)) (Variables|Default|GetOriginalRotation) (Utilities|Time|GetWorldDeltaSeconds) 1.0) false false))

(event OnComponentEndOverlap(Sponge3Box)
  (params (OverlappedComponent :type Primitive%20Component%20Object%20Reference) (OtherActor :type Actor%20Object%20Reference) (OtherComp :type Primitive%20Component%20Object%20Reference) (OtherBodyIndex :type Integer))
  ;[1 1 1] Return sponge 3 to original rotation when they arent touching it
  (Utilities|Casting|CastToFlyingPawn OtherActor)
  (Transformation|SetWorldRotation (Variables|Default|GetSponge3) (Math|Interpolation|RInterpTo (Transformation|GetWorldRotation (Variables|Default|GetSponge3)) (Variables|Default|GetOriginalRotation) (Utilities|Time|GetWorldDeltaSeconds) 1.0) false false))

(event OnComponentEndOverlap(Sponge4Box)
  (params (OverlappedComponent :type Primitive%20Component%20Object%20Reference) (OtherActor :type Actor%20Object%20Reference) (OtherComp :type Primitive%20Component%20Object%20Reference) (OtherBodyIndex :type Integer))
  ;[1 1 1] Return sponge 4 to original rotation when they arent touching it
  (Utilities|Casting|CastToFlyingPawn OtherActor)
  (Transformation|SetWorldRotation (Variables|Default|GetSponge4) (Math|Interpolation|RInterpTo (Transformation|GetWorldRotation (Variables|Default|GetSponge4)) (Variables|Default|GetOriginalRotation) (Utilities|Time|GetWorldDeltaSeconds) 1.0) false false))

(event EventBeginPlay
  ;[1 1 1] Create array from sponges, get original rotations for them and set reference to flying pawn
  (Variables|Default|SetSpongeArray (Utilities|Array|MakeArray (Variables|Default|GetSponge1) (Variables|Default|GetSponge2) (Variables|Default|GetSponge3) (Variables|Default|GetSponge4)))
  (Variables|Default|SetOriginalRotation (Transformation|GetWorldRotation (Variables|Default|GetSponge1)))
  (bind _asflying_pawn (Utilities|Casting|CastToFlyingPawn (Game|Player|GetPlayerPawn 0)))
  (Variables|Default|SetFlyingPawnReference _asflying_pawn))

(fn ConstructionScript)