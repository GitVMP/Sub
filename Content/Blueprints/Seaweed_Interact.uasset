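; Seaweed actor with four seaweed pieces and an interact widget for the player's FlyingPawn.
; Tick turns the widget toward the pawn's camera, tints whatever widget its WidgetInteraction hovers visible, otherwise hides InteractSeaweed, and updates the pawn's HoveringAWidget flag.
; When the pawn leaves a piece's box, a single RInterpTo step nudges that piece toward Seaweed1's starting rotation; nothing here bends the seaweed.
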(event OnComponentEndOverlap(Seaweed2Box)
  (params (OverlappedComponent :type Primitive%20Component%20Object%20Reference) (OtherActor :type Actor%20Object%20Reference) (OtherComp :type Primitive%20Component%20Object%20Reference) (OtherBodyIndex :type Integer))
  ;[1 1 1] Return seaweed 2 to original rotation when they arent touching it
  (Utilities|Casting|CastToFlyingPawn OtherActor)
  (Transformation|SetWorldRotation (Variables|Default|GetSeaweed2) (Math|Interpolation|RInterpTo (Transformation|GetWorldRotation (Variables|Default|GetSeaweed2)) (Variables|Default|GetOriginalRotation) (Utilities|Time|GetWorldDeltaSeconds) 1.0) false false))

(event OnComponentEndOverlap(Seaweed3Box)
  (params (OverlappedComponent :type Primitive%20Component%20Object%20Reference) (OtherActor :type Actor%20Object%20Reference) (OtherComp :type Primitive%20Component%20Object%20Reference) (OtherBodyIndex :type Integer))
  ;[1 1 1] Return seaweed 3 to original rotation when they arent touching it
  (Utilities|Casting|CastToFlyingPawn OtherActor)
  (Transformation|SetWorldRotation (Variables|Default|GetSeaweed3) (Math|Interpolation|RInterpTo (Transformation|GetWorldRotation (Variables|Default|GetSeaweed3)) (Variables|Default|GetOriginalRotation) (Utilities|Time|GetWorldDeltaSeconds) 1.0) false false))

(event OnComponentEndOverlap(Seaweed4Box)
  (params (OverlappedComponent :type Primitive%20Component%20Object%20Reference) (OtherActor :type Actor%20Object%20Reference) (OtherComp :type Primitive%20Component%20Object%20Reference) (OtherBodyIndex :type Integer))
  ;[1 1 1] Return seaweed 4 to original rotation when they arent touching it
  (Utilities|Casting|CastToFlyingPawn OtherActor)
  (Transformation|SetWorldRotation (Variables|Default|GetSeaweed4) (Math|Interpolation|RInterpTo (Transformation|GetWorldRotation (Variables|Default|GetSeaweed4)) (Variables|Default|GetOriginalRotation) (Utilities|Time|GetWorldDeltaSeconds) 1.0) false false))

(event OnComponentEndOverlap(Seaweed1Box)
  (params (OverlappedComponent :type Primitive%20Component%20Object%20Reference) (OtherActor :type Actor%20Object%20Reference) (OtherComp :type Primitive%20Component%20Object%20Reference) (OtherBodyIndex :type Integer))
  ;[1 1 1] Return seaweed 1 to original rotation when they arent touching it
  (Utilities|Casting|CastToFlyingPawn OtherActor)
  (Transformation|SetWorldRotation (Variables|Default|GetSeaweed1) (Math|Interpolation|RInterpTo (Transformation|GetWorldRotation (Variables|Default|GetSeaweed1)) (Variables|Default|GetOriginalRotation) (Utilities|Time|GetWorldDeltaSeconds) 1.0) false false))

(event EventBeginPlay
  ;[1 1 1] Create array of seaweed, get original rotation of one and get a reference to the flying pawn
  (Variables|Default|SetSeaweedArray (Utilities|Array|MakeArray (Variables|Default|GetSeaweed1) (Variables|Default|GetSeaweed2) (Variables|Default|GetSeaweed3) (Variables|Default|GetSeaweed4)))
  (Variables|Default|SetOriginalRotation (Transformation|GetWorldRotation (Variables|Default|GetSeaweed1)))
  (bind _asflying_pawn (Utilities|Casting|CastToFlyingPawn (Game|Player|GetPlayerPawn 0)))
  (Variables|Default|SetFlyingPawnReference _asflying_pawn))

(event EventTick
  (params (DeltaSeconds :type Float%20%28single-precision%29))
  (bind _flyingpawnreference (Variables|Default|GetFlyingPawnReference))
  (bind _widgetinteraction (Variables|/Game/FlyingBP/Blueprints/FlyingPawn.FlyingPawn_C|GetWidgetInteraction _flyingpawnreference))
  (bind _returnvalue (Class|WidgetInteractionComponent|GetHoveredWidgetComponent _widgetinteraction))
  ;[1 1 1] Show interact widget when they are looking at the seaweed and face it towards the player
  (Transformation|SetWorldRotation (Variables|Default|GetInteract_Seaweed) (Math|Rotator|FindLookatRotation (Transformation|GetWorldLocation (Variables|Default|GetInteract_Seaweed)) (Transformation|GetWorldLocation (Variables|/Game/FlyingBP/Blueprints/FlyingPawn.FlyingPawn_C|GetCamera (Variables|Default|GetFlyingPawnReference)))) false false)
  (if (Utilities|Enum|NotEqual(Enum) (Utilities|GetDisplayName _returnvalue) "") ; Check if they are hovering a widget. If yes, display that widget
    (Class|WidgetComponent|SetTintColorandOpacity _returnvalue "(R=1.000000,G=1.000000,B=1.000000,A=1.000000)") ; Show the widget that is being hovered
    (Variables|/Game/FlyingBP/Blueprints/FlyingPawn.FlyingPawn_C|SetHoveringAWidget? (Variables|Default|GetFlyingPawnReference) true)
    (else
      (Class|WidgetComponent|SetTintColorandOpacity (Variables|Default|GetInteract_Seaweed) "(R=0.000000,G=0.000000,B=0.000000,A=0.000000)") ; Hide all widgets that arent being hovered  (Connect all interact components here)
      (Variables|/Game/FlyingBP/Blueprints/FlyingPawn.FlyingPawn_C|SetHoveringAWidget? (Variables|Default|GetFlyingPawnReference) false))))

(fn ConstructionScript)