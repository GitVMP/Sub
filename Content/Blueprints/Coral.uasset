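; Coral prop that simulates physics only while a FlyingPawn is inside its trigger volume.
; Begin overlap on Coral_Trigger turns on physics simulation and physics-only collision for the Coral component.
; End overlap turns simulation off and removes collision, and overlaps by any other actor type are ignored.
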(event OnComponentBeginOverlap(Coral_Trigger)
  (params (OverlappedComponent :type Primitive%20Component%20Object%20Reference) (OtherActor :type Actor%20Object%20Reference) (OtherComp :type Primitive%20Component%20Object%20Reference) (OtherBodyIndex :type Integer) (bFromSweep :type Boolean) (SweepResult :type Hit%20Result%20Structure%20%28by%20ref%29))
  (Utilities|Casting|CastToFlyingPawn OtherActor)
  (Physics|SetSimulatePhysics (Variables|Default|GetCoral) true)
  (Collision|SetCollisionEnabled (Variables|Default|GetCoral) "PhysicsOnly"))

(event OnComponentEndOverlap(Coral_Trigger)
  (params (OverlappedComponent :type Primitive%20Component%20Object%20Reference) (OtherActor :type Actor%20Object%20Reference) (OtherComp :type Primitive%20Component%20Object%20Reference) (OtherBodyIndex :type Integer))
  (Utilities|Casting|CastToFlyingPawn OtherActor)
  (Physics|SetSimulatePhysics (Variables|Default|GetCoral) false)
  (Collision|SetCollisionEnabled (Variables|Default|GetCoral) "NoCollision"))

(fn ConstructionScript)