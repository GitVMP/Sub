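; Interactable sponge actor with four sponge meshes and an interact widget that turns to face the FlyingPawn's camera.
; Tick shows whichever widget the pawn's WidgetInteraction hovers, otherwise hides InteractSponge, and updates the pawn's HoveringAWidget flag.
; When the pawn leaves a sponge's box, that sponge takes a single RInterpTo step toward Sponge1's starting rotation, which all four share as their target.
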(event OnComponentEndOverlap(Sponge1Box)
  (params (OverlappedComponent :type Primitive%20Component%20Object%20Reference) (OtherActor :type Actor%20Object%20Reference) (OtherComp :type Primitive%20Component%20Object%20Reference) (OtherBodyIndex :type Integer))
  ;[1 1 1] Return sponge 1 to original rotation when they arent touching it
  (Utilities|Casting|CastToFlyingPawn OtherActor)
  (Transformation|SetWorldRotation (Variables|Default|GetSponge1) (Math|Interpolation|RInterpTo (Transformation|GetWorldRotation (Variables|Default|GetSponge1)) (Variables|Default|GetOriginalRotation) (Utilities|Time|GetWorldDeltaSeconds) 1.0) false false))

(event OnComponentEndOverlap(Sponge2Box)
  (params (OverlappedComponent :type Primitive%20Component%20Object%20Reference) (OtherActor :type Actor%20Object%20Reference) (OtherComp :type Primitive%20Component%20Object%20Reference) (OtherBodyIndex :type Integer))
  ;[1 1 1] Return sponge 2 to original rotation when they arent touching it
  (Utilities|Casting|CastToFlyingPawn OtherActor)
  (Transformation|SetWorldRotation (Variables|Default|GetSponge2) (Math|Interpolation|RInterpTo (Transformation|GetWorldRotation (Variables|Default|GetSponge2)) (Variables|Default|GetOriginalRotation) (Utilities|Time|GetWorldDeltaSeconds) 1.0) false false))

(event OnComponentEndOverlap(Sponge3Box)
  (params (OverlappedComponent :type Primitive%20Component%20Object%20Reference) (OtherActor :type Actor%20Object%20Reference) (OtherComp :type Primitive%20Component%20Object%20Reference) (OtherBodyIndex :type Integer))
  ;[1 1 1] Return sponge 3 to original rotation when they arent touching it
  (Utilities|Casting|CastToFlyingPawn OtherActor)
  (Transformation|SetWorldRotation (Variables|Default|GetSponge3) (Math|Interpolation|RInterpTo (Transformation|GetWorldRotation (Variables|Default|GetSponge3)) (Variables|Default|GetOriginalRotation) (Utilities|Time|GetWorldDeltaSeconds) 1.0) false false))

(event OnComponentEndOverlap(Sponge4Box)
  (params (OverlappedComponent :type Primitive%20Component%20Object%20Reference) (OtherActor :type Actor%20Object%20Reference) (OtherComp :type Primitive%20Component%20Object%20Reference) (OtherBodyIndex :type Integer))
  ;[1 1 1] Return sponge 4 to original rotation when they arent touching it
  (Utilities|Casting|CastToFlyingPawn OtherActor)
  (Transformation|SetWorldRotation (Variables|Default|GetSponge4) (Math|Interpolation|RInterpTo (Transformation|GetWorldRotation (Variables|Default|GetSponge4)) (Variables|Default|GetOriginalRotation) (Utilities|Time|GetWorldDeltaSeconds) 1.0) false false))

(event EventBeginPlay
  ;[1 1 1] Create array from sponges, get original rotations for them and set reference to flying pawn
  (Variables|Default|SetSpongeArray (Utilities|Array|MakeArray (Variables|Default|GetSponge1) (Variables|Default|GetSponge2) (Variables|Default|GetSponge3) (Variables|Default|GetSponge4)))
  (Variables|Default|SetOriginalRotation (Transformation|GetWorldRotation (Variables|Default|GetSponge1)))
  (bind _asflying_pawn (Utilities|Casting|CastToFlyingPawn (Game|Player|GetPlayerPawn 0)))
  (Variables|Default|SetFlyingPawnReference _asflying_pawn))

(event EventTick
  (params (DeltaSeconds :type Float%20%28single-precision%29))
  (bind _flyingpawnreference (Variables|Default|GetFlyingPawnReference))
  (bind _widgetinteraction (Variables|/Game/FlyingBP/Blueprints/FlyingPawn.FlyingPawn_C|GetWidgetInteraction _flyingpawnreference))
  (bind _returnvalue (Class|WidgetInteractionComponent|GetHoveredWidgetComponent _widgetinteraction))
  ;[1 1 1] Show interact widget when player is looking at the sponge and set to always face towards their camera
  (Transformation|SetWorldRotation (Variables|Default|GetInteract_Sponge) (Math|Rotator|FindLookatRotation (Transformation|GetWorldLocation (Variables|Default|GetInteract_Sponge)) (Transformation|GetWorldLocation (Variables|/Game/FlyingBP/Blueprints/FlyingPawn.FlyingPawn_C|GetCamera (Variables|Default|GetFlyingPawnReference)))) false false)
  (if (Utilities|Enum|NotEqual(Enum) (Utilities|GetDisplayName _returnvalue) "") ; Check if they are hovering a widget. If yes, display that widget
    (Class|WidgetComponent|SetTintColorandOpacity _returnvalue "(R=1.000000,G=1.000000,B=1.000000,A=1.000000)") ; Show the widget that is being hovered
    (Variables|/Game/FlyingBP/Blueprints/FlyingPawn.FlyingPawn_C|SetHoveringAWidget? (Variables|Default|GetFlyingPawnReference) true)
    (else
      (Class|WidgetComponent|SetTintColorandOpacity (Variables|Default|GetInteract_Sponge) "(R=0.000000,G=0.000000,B=0.000000,A=0.000000)") ; Hide all widgets that arent being hovered  (Connect all interact components here)
      (Variables|/Game/FlyingBP/Blueprints/FlyingPawn.FlyingPawn_C|SetHoveringAWidget? (Variables|Default|GetFlyingPawnReference) false))))

(fn ConstructionScript)